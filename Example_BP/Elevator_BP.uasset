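; Player-controlled elevator actor that moves and rotates while keys are held inside its trigger box.
; Box overlap enables input, unhides tagged actors and switches LensFlare_BP ones on; exit reverses this.
; Number keys raise, lower and rotate the root, and E shifts it sideways.
; Timelines serve as hold-to-move tickers adding fixed, frame-rate-dependent steps, with sweep only on descent.
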(event OnComponentBeginOverlap(Box)
  (params (OverlappedComponent :type Primitive%20Component%20Object%20Reference) (OtherActor :type Actor%20Object%20Reference) (OtherComp :type Primitive%20Component%20Object%20Reference) (OtherBodyIndex :type Integer) (bFromSweep :type Boolean) (SweepResult :type Hit%20Result%20Structure%20%28by%20ref%29))
  (Input|EnableInput (Game|GetPlayerController 0))
  (bind _outactors (Actor|GetAllActorswithTag (Variables|Default|GetTag)))
  (for _array_element _outactors
    (Rendering|SetActorHiddenInGame _array_element false)
    (bind _aslens_flare_bp (Utilities|Casting|CastToLensFlare_BP _array_element))
    (Variables|/Game/LensFlareEff/Blueprints/LensFlare_BP.LensFlare_BP_C|SetOnOff _aslens_flare_bp true)))

(event OnComponentEndOverlap(Box)
  (params (OverlappedComponent :type Primitive%20Component%20Object%20Reference) (OtherActor :type Actor%20Object%20Reference) (OtherComp :type Primitive%20Component%20Object%20Reference) (OtherBodyIndex :type Integer))
  (Input|DisableInput (Game|GetPlayerController 0))
  (bind _outactors (Actor|GetAllActorswithTag (Variables|Default|GetTag)))
  (for _array_element _outactors
    (Rendering|SetActorHiddenInGame _array_element true)
    (bind _aslens_flare_bp (Utilities|Casting|CastToLensFlare_BP _array_element))
    (Variables|/Game/LensFlareEff/Blueprints/LensFlare_BP.LensFlare_BP_C|SetOnOff _aslens_flare_bp false)))

(event Input|KeyboardEvents|1
  (params (Key :type Key%20Structure :default "None"))
  (:Pressed
    (Timeline|Timeline_0 PlayFromStart
      (:Update
        (Transformation|AddLocalOffset (Variables|Default|GetDefaultSceneRoot) "0, 0,12.000000" false false))))
  (:Released
    (Timeline|Timeline_0 Stop)))

(event Input|KeyboardEvents|2
  (params (Key :type Key%20Structure :default "None"))
  (:Pressed
    (Timeline|Timeline_1 PlayFromStart
      (:Update
        (Transformation|AddLocalOffset (Variables|Default|GetDefaultSceneRoot) "0, 0,-5.000000" true false))))
  (:Released
    (Timeline|Timeline_1 Stop)))

(event Input|KeyboardEvents|3
  (params (Key :type Key%20Structure :default "None"))
  (:Pressed
    (Timeline|Timeline_2 PlayFromStart
      (:Update
        (Transformation|AddLocalRotation (Variables|Default|GetDefaultSceneRoot) "0,-1.000000, 0" false false))))
  (:Released
    (Timeline|Timeline_2 Stop)))

(event Input|KeyboardEvents|4
  (params (Key :type Key%20Structure :default "None"))
  (:Pressed
    (Timeline|Timeline_3 PlayFromStart
      (:Update
        (Transformation|AddLocalRotation (Variables|Default|GetDefaultSceneRoot) "0,1.000000, 0" false false))))
  (:Released
    (Timeline|Timeline_3 Stop)))

(event Input|KeyboardEvents|E
  (params (Key :type Key%20Structure :default "None"))
  (:Pressed
    (Timeline|Timeline_4 PlayFromStart
      (:Update
        (Transformation|AddLocalOffset (Variables|Default|GetDefaultSceneRoot) "0.000000,-3.000000,0.000000" false false))))
  (:Released
    (Timeline|Timeline_4 Stop)))

(fn ConstructionScript)