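; Lens flare actor that draws screen-space flare elements for a light source, with an optional point light.
; On BeginPlay it creates and initializes one widget per FlareElements entry, each with a dynamic material.
; Each Tick, camera distance checks and a visibility line trace set each widget's occlusion multiplier.
; A curve-driven timeline can pulse flares and light color (Shine), and moveable flares follow the actor's transform.
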(event EventBeginPlay
  (CallFunction|InitiateFlares))

(event EventTick
  (params (DeltaSeconds :type Float%20%28single-precision%29))
  (bind _timeline_0 (Variables|Default|GetTimeline_0))
  (Utilities|FlowControl|Sequence
    (:then_0
      (CallFunction|UpdateFlareVisibility)
      (if (Variables|Global|GetFlare%20Moveable)
        (for _array_element (Variables|FlareElementList|GetFlare%20Elements)
          (Variables|/Game/LensFlareEff/Blueprints/FlareWidget.FlareWidget_C|SetParentLocation (.FlareWidget (Utilities|Struct|BreakStruct_FlareItem _array_element)) (Math|Transform|TransformLocation (Transformation|GetActorTransform) (Variables|Global|GetFlare%20Offset))))))
    (:then_1
      (Components|Timeline|SetPlayRate _timeline_0 (Variables|Global|GetShineRate))
      (Components|Timeline|SetTimelineLength _timeline_0 (Variables|Global|GetShineLength))
      (Class|TimelineComponent|SetFloatCurve _timeline_0 (Variables|Global|GetShineCurve) "ShineCurver")
      (bind _shinecurver (Timeline|Timeline_0 Play)
        (:Update
          (Variables|Default|SetShineLighting _shinecurver))))))

(fn ConstructionScript)

(fn UpdateFlareVisibility
  (bind _returnvalue (Game|GetPlayerController 0))
  (bind _shine (Variables|Global|GetShine))
  (bind _widgetlist (Variables|Default|GetWidgetList))
  (bind _onoff (Variables|Global|GetOnOff))
  (bind _use_pointlight (Variables|Global|GetUse%20PointLight))
  (bind _pointlight (Variables|Default|GetPointLight))
  (bind _shinelighting (Variables|Default|GetShineLighting))
  (bind _lightcolor (Variables|Default|GetlightColor))
  (bind _returnvalue_2 (Math|Conversions|ToLinearColor(Color) _lightcolor))
  (bind _playercameramanager (Variables|/Script/Engine.PlayerController|GetPlayerCameraManager _returnvalue))
  (bind _returnvalue_3 (Transformation|GetDistanceTo _playercameramanager))
  (bind _returnvalue_4 (Math|Conversions|ToVector(LinearColor) _returnvalue_2))
  (bind _returnvalue_5 (Math|Vector|Lerp(Vector) "0, 0, 0" _returnvalue_4 _shinelighting))
  (bind _returnvalue_6 (Math|Conversions|ToLinearColor(Vector) _returnvalue_5))
  ;[1 1 1] First check the source BP distance to the camera.  If it's past max, kill the check completely
  (if (> _returnvalue_3 (Variables|Global|GetGlobal%20Maximum%20Distance))
    ;[1 1 1] If it's beyond max range clear the occlusion controlling variable in each flare element
    (for _array_element _widgetlist :!label _label
      (Variables|/Game/LensFlareEff/Blueprints/FlareWidget.FlareWidget_C|SetOcclusionMult _array_element 0.0)
      (if _onoff
        (if _use_pointlight
          (if _shine
            (Rendering|Components|Light|SetLightColor _pointlight _returnvalue_6 true)
            (else
              (Rendering|Components|Light|SetLightColor _pointlight (Math|Conversions|ToLinearColor(Color) _lightcolor) true)))
          (else
            (Rendering|SetVisibility _pointlight false false :!label _label_2)))
        (else
          (goto _label_2))))
    (else
      ;[1 1 1] Establish if the source is then visible
      (bind _returnvalue_7 (Collision|LineTraceByChannel (Transformation|GetWorldLocation (Variables|Default|GetDefaultSceneRoot)) (Transformation|GetWorldLocation (Variables|/Script/Engine.PlayerCameraManager|GetTransformComponent _playercameramanager)) "TraceTypeQuery1" false 0 "None"))
      ;[1 1 1] Then if not visible occlude
      (if _returnvalue_7
        (goto _label)
        (else
          ;[1 1 1] Then per element, check the fade distance, and adjust accordingly
          (for _array_element_2 _widgetlist
            (if _onoff
              (if (> _returnvalue_3 (Variables|/Game/LensFlareEff/Blueprints/FlareWidget.FlareWidget_C|GetFadeDistance _array_element_2))
                (Variables|/Game/LensFlareEff/Blueprints/FlareWidget.FlareWidget_C|SetOcclusionMult _array_element_2 0.0 :!label _label_3)
                (elif _shine
                  (Variables|/Game/LensFlareEff/Blueprints/FlareWidget.FlareWidget_C|SetOcclusionMult _array_element_2 _shinelighting)
                  (Rendering|SetVisibility _pointlight _use_pointlight false)
                  (if _use_pointlight
                    (Rendering|Components|Light|SetLightColor _pointlight _returnvalue_6 true))
                  (else
                    (Variables|/Game/LensFlareEff/Blueprints/FlareWidget.FlareWidget_C|SetOcclusionMult _array_element_2 1.0)
                    (Utilities|FlowControl|DoOnce false
                      (:Completed
                        (Rendering|Components|Light|SetLightColor _pointlight (Math|Conversions|ToLinearColor(Color) _lightcolor) true)
                        (Rendering|SetVisibility _pointlight _use_pointlight false))))))
              (else
                (Utilities|FlowControl|Sequence
                  (:then_0
                    (goto _label_3))
                  (:then_1
                    (Rendering|SetVisibility _pointlight false false)))))))))))

(fn InitiateFlares
  (bind _flare_elements (Variables|FlareElementList|GetFlare%20Elements))
  ;[1 1 1] For Each Flare Element
  (for (_array_element _array_index) _flare_elements
    ;[1 1 1] Create new flare element widget
    (bind _returnvalue (UserInterface|CreateWidget "/Game/LensFlareEff/Blueprints/FlareWidget.FlareWidget_C" (Game|GetPlayerController 0)))
    ;[1 1 1] Add that widget to the flare element struct
    (Utilities|Array|SetArrayElem _flare_elements _array_index (Utilities|Struct|MakeStruct_FlareItem (.Color (Utilities|Struct|BreakStruct_FlareItem _array_element)) _returnvalue (.FlareLocation (Utilities|Struct|BreakStruct_FlareItem _array_element)) (.IsMaterialAdditive (Utilities|Struct|BreakStruct_FlareItem _array_element)) (.FadeoutEdgeDistance (Utilities|Struct|BreakStruct_FlareItem _array_element)) (.ElementMaximumDistance (Utilities|Struct|BreakStruct_FlareItem _array_element)) (.FadeOut_EnableShrinking (Utilities|Struct|BreakStruct_FlareItem _array_element)) true (.FadeOut_FlareLocation (Utilities|Struct|BreakStruct_FlareItem _array_element)) (.Material (Utilities|Struct|BreakStruct_FlareItem _array_element)) (.ScreenPositionOffset (Utilities|Struct|BreakStruct_FlareItem _array_element)) (.GlobalSizeMultiplier (Utilities|Struct|BreakStruct_FlareItem _array_element)) (.InitialSpriteAngle (Utilities|Struct|BreakStruct_FlareItem _array_element)) (.ActiveRotationAmount (Utilities|Struct|BreakStruct_FlareItem _array_element)) (.EnableOrbitRotation (Utilities|Struct|BreakStruct_FlareItem _array_element)) (.EnablesLocationScaling (Utilities|Struct|BreakStruct_FlareItem _array_element)) (.LocationScalingInfluence (Utilities|Struct|BreakStruct_FlareItem _array_element)) (.LocationScalingCenterSize (Utilities|Struct|BreakStruct_FlareItem _array_element)) (.LocationScalingEdgeSize (Utilities|Struct|BreakStruct_FlareItem _array_element)) (.EnableLocationBasedOpacity (Utilities|Struct|BreakStruct_FlareItem _array_element)) (.LocOpacityCenterOpacity (Utilities|Struct|BreakStruct_FlareItem _array_element)) (.LocOpacityEdgeOpacity (Utilities|Struct|BreakStruct_FlareItem _array_element)) (.LocOpacityInfluence (Utilities|Struct|BreakStruct_FlareItem _array_element))))
    ;[1 1 1] Initialize each widget. This means passing most of the element struct information, and adding the material, setting the color and a few other things
    (if (Utilities|IsValid (.Material (Utilities|Struct|BreakStruct_FlareItem (Utilities|Struct|MakeStruct_FlareItem (.Color (Utilities|Struct|BreakStruct_FlareItem _array_element)) _returnvalue (.FlareLocation (Utilities|Struct|BreakStruct_FlareItem _array_element)) (.IsMaterialAdditive (Utilities|Struct|BreakStruct_FlareItem _array_element)) (.FadeoutEdgeDistance (Utilities|Struct|BreakStruct_FlareItem _array_element)) (.ElementMaximumDistance (Utilities|Struct|BreakStruct_FlareItem _array_element)) (.FadeOut_EnableShrinking (Utilities|Struct|BreakStruct_FlareItem _array_element)) true (.FadeOut_FlareLocation (Utilities|Struct|BreakStruct_FlareItem _array_element)) (.Material (Utilities|Struct|BreakStruct_FlareItem _array_element)) (.ScreenPositionOffset (Utilities|Struct|BreakStruct_FlareItem _array_element)) (.GlobalSizeMultiplier (Utilities|Struct|BreakStruct_FlareItem _array_element)) (.InitialSpriteAngle (Utilities|Struct|BreakStruct_FlareItem _array_element)) (.ActiveRotationAmount (Utilities|Struct|BreakStruct_FlareItem _array_element)) (.EnableOrbitRotation (Utilities|Struct|BreakStruct_FlareItem _array_element)) (.EnablesLocationScaling (Utilities|Struct|BreakStruct_FlareItem _array_element)) (.LocationScalingInfluence (Utilities|Struct|BreakStruct_FlareItem _array_element)) (.LocationScalingCenterSize (Utilities|Struct|BreakStruct_FlareItem _array_element)) (.LocationScalingEdgeSize (Utilities|Struct|BreakStruct_FlareItem _array_element)) (.EnableLocationBasedOpacity (Utilities|Struct|BreakStruct_FlareItem _array_element)) (.LocOpacityCenterOpacity (Utilities|Struct|BreakStruct_FlareItem _array_element)) (.LocOpacityEdgeOpacity (Utilities|Struct|BreakStruct_FlareItem _array_element)) (.LocOpacityInfluence (Utilities|Struct|BreakStruct_FlareItem _array_element))))))
      (bind _returnvalue_2 (Rendering|Material|CreateDynamicMaterialInstance (.Material (Utilities|Struct|BreakStruct_FlareItem (Utilities|Struct|MakeStruct_FlareItem (.Color (Utilities|Struct|BreakStruct_FlareItem _array_element)) _returnvalue (.FlareLocation (Utilities|Struct|BreakStruct_FlareItem _array_element)) (.IsMaterialAdditive (Utilities|Struct|BreakStruct_FlareItem _array_element)) (.FadeoutEdgeDistance (Utilities|Struct|BreakStruct_FlareItem _array_element)) (.ElementMaximumDistance (Utilities|Struct|BreakStruct_FlareItem _array_element)) (.FadeOut_EnableShrinking (Utilities|Struct|BreakStruct_FlareItem _array_element)) true (.FadeOut_FlareLocation (Utilities|Struct|BreakStruct_FlareItem _array_element)) (.Material (Utilities|Struct|BreakStruct_FlareItem _array_element)) (.ScreenPositionOffset (Utilities|Struct|BreakStruct_FlareItem _array_element)) (.GlobalSizeMultiplier (Utilities|Struct|BreakStruct_FlareItem _array_element)) (.InitialSpriteAngle (Utilities|Struct|BreakStruct_FlareItem _array_element)) (.ActiveRotationAmount (Utilities|Struct|BreakStruct_FlareItem _array_element)) (.EnableOrbitRotation (Utilities|Struct|BreakStruct_FlareItem _array_element)) (.EnablesLocationScaling (Utilities|Struct|BreakStruct_FlareItem _array_element)) (.LocationScalingInfluence (Utilities|Struct|BreakStruct_FlareItem _array_element)) (.LocationScalingCenterSize (Utilities|Struct|BreakStruct_FlareItem _array_element)) (.LocationScalingEdgeSize (Utilities|Struct|BreakStruct_FlareItem _array_element)) (.EnableLocationBasedOpacity (Utilities|Struct|BreakStruct_FlareItem _array_element)) (.LocOpacityCenterOpacity (Utilities|Struct|BreakStruct_FlareItem _array_element)) (.LocOpacityEdgeOpacity (Utilities|Struct|BreakStruct_FlareItem _array_element)) (.LocOpacityInfluence (Utilities|Struct|BreakStruct_FlareItem _array_element))))) "None" :!class /Script/Engine.KismetMaterialLibrary))
      (Variables|/Game/LensFlareEff/Blueprints/FlareWidget.FlareWidget_C|SetCurrentMaterial (.FlareWidget (Utilities|Struct|BreakStruct_FlareItem (Utilities|Struct|MakeStruct_FlareItem (.Color (Utilities|Struct|BreakStruct_FlareItem _array_element)) _returnvalue (.FlareLocation (Utilities|Struct|BreakStruct_FlareItem _array_element)) (.IsMaterialAdditive (Utilities|Struct|BreakStruct_FlareItem _array_element)) (.FadeoutEdgeDistance (Utilities|Struct|BreakStruct_FlareItem _array_element)) (.ElementMaximumDistance (Utilities|Struct|BreakStruct_FlareItem _array_element)) (.FadeOut_EnableShrinking (Utilities|Struct|BreakStruct_FlareItem _array_element)) true (.FadeOut_FlareLocation (Utilities|Struct|BreakStruct_FlareItem _array_element)) (.Material (Utilities|Struct|BreakStruct_FlareItem _array_element)) (.ScreenPositionOffset (Utilities|Struct|BreakStruct_FlareItem _array_element)) (.GlobalSizeMultiplier (Utilities|Struct|BreakStruct_FlareItem _array_element)) (.InitialSpriteAngle (Utilities|Struct|BreakStruct_FlareItem _array_element)) (.ActiveRotationAmount (Utilities|Struct|BreakStruct_FlareItem _array_element)) (.EnableOrbitRotation (Utilities|Struct|BreakStruct_FlareItem _array_element)) (.EnablesLocationScaling (Utilities|Struct|BreakStruct_FlareItem _array_element)) (.LocationScalingInfluence (Utilities|Struct|BreakStruct_FlareItem _array_element)) (.LocationScalingCenterSize (Utilities|Struct|BreakStruct_FlareItem _array_element)) (.LocationScalingEdgeSize (Utilities|Struct|BreakStruct_FlareItem _array_element)) (.EnableLocationBasedOpacity (Utilities|Struct|BreakStruct_FlareItem _array_element)) (.LocOpacityCenterOpacity (Utilities|Struct|BreakStruct_FlareItem _array_element)) (.LocOpacityEdgeOpacity (Utilities|Struct|BreakStruct_FlareItem _array_element)) (.LocOpacityInfluence (Utilities|Struct|BreakStruct_FlareItem _array_element))))) _returnvalue_2)
      (elif (.IsMaterialAdditive (Utilities|Struct|BreakStruct_FlareItem (Utilities|Struct|MakeStruct_FlareItem (.Color (Utilities|Struct|BreakStruct_FlareItem _array_element)) _returnvalue (.FlareLocation (Utilities|Struct|BreakStruct_FlareItem _array_element)) (.IsMaterialAdditive (Utilities|Struct|BreakStruct_FlareItem _array_element)) (.FadeoutEdgeDistance (Utilities|Struct|BreakStruct_FlareItem _array_element)) (.ElementMaximumDistance (Utilities|Struct|BreakStruct_FlareItem _array_element)) (.FadeOut_EnableShrinking (Utilities|Struct|BreakStruct_FlareItem _array_element)) true (.FadeOut_FlareLocation (Utilities|Struct|BreakStruct_FlareItem _array_element)) (.Material (Utilities|Struct|BreakStruct_FlareItem _array_element)) (.ScreenPositionOffset (Utilities|Struct|BreakStruct_FlareItem _array_element)) (.GlobalSizeMultiplier (Utilities|Struct|BreakStruct_FlareItem _array_element)) (.InitialSpriteAngle (Utilities|Struct|BreakStruct_FlareItem _array_element)) (.ActiveRotationAmount (Utilities|Struct|BreakStruct_FlareItem _array_element)) (.EnableOrbitRotation (Utilities|Struct|BreakStruct_FlareItem _array_element)) (.EnablesLocationScaling (Utilities|Struct|BreakStruct_FlareItem _array_element)) (.LocationScalingInfluence (Utilities|Struct|BreakStruct_FlareItem _array_element)) (.LocationScalingCenterSize (Utilities|Struct|BreakStruct_FlareItem _array_element)) (.LocationScalingEdgeSize (Utilities|Struct|BreakStruct_FlareItem _array_element)) (.EnableLocationBasedOpacity (Utilities|Struct|BreakStruct_FlareItem _array_element)) (.LocOpacityCenterOpacity (Utilities|Struct|BreakStruct_FlareItem _array_element)) (.LocOpacityEdgeOpacity (Utilities|Struct|BreakStruct_FlareItem _array_element)) (.LocOpacityInfluence (Utilities|Struct|BreakStruct_FlareItem _array_element)))))
        (bind _returnvalue_3 (Rendering|Material|CreateDynamicMaterialInstance 0 "None" :!class /Script/Engine.KismetMaterialLibrary))
        (Variables|/Game/LensFlareEff/Blueprints/FlareWidget.FlareWidget_C|SetCurrentMaterial (.FlareWidget (Utilities|Struct|BreakStruct_FlareItem (Utilities|Struct|MakeStruct_FlareItem (.Color (Utilities|Struct|BreakStruct_FlareItem _array_element)) _returnvalue (.FlareLocation (Utilities|Struct|BreakStruct_FlareItem _array_element)) (.IsMaterialAdditive (Utilities|Struct|BreakStruct_FlareItem _array_element)) (.FadeoutEdgeDistance (Utilities|Struct|BreakStruct_FlareItem _array_element)) (.ElementMaximumDistance (Utilities|Struct|BreakStruct_FlareItem _array_element)) (.FadeOut_EnableShrinking (Utilities|Struct|BreakStruct_FlareItem _array_element)) true (.FadeOut_FlareLocation (Utilities|Struct|BreakStruct_FlareItem _array_element)) (.Material (Utilities|Struct|BreakStruct_FlareItem _array_element)) (.ScreenPositionOffset (Utilities|Struct|BreakStruct_FlareItem _array_element)) (.GlobalSizeMultiplier (Utilities|Struct|BreakStruct_FlareItem _array_element)) (.InitialSpriteAngle (Utilities|Struct|BreakStruct_FlareItem _array_element)) (.ActiveRotationAmount (Utilities|Struct|BreakStruct_FlareItem _array_element)) (.EnableOrbitRotation (Utilities|Struct|BreakStruct_FlareItem _array_element)) (.EnablesLocationScaling (Utilities|Struct|BreakStruct_FlareItem _array_element)) (.LocationScalingInfluence (Utilities|Struct|BreakStruct_FlareItem _array_element)) (.LocationScalingCenterSize (Utilities|Struct|BreakStruct_FlareItem _array_element)) (.LocationScalingEdgeSize (Utilities|Struct|BreakStruct_FlareItem _array_element)) (.EnableLocationBasedOpacity (Utilities|Struct|BreakStruct_FlareItem _array_element)) (.LocOpacityCenterOpacity (Utilities|Struct|BreakStruct_FlareItem _array_element)) (.LocOpacityEdgeOpacity (Utilities|Struct|BreakStruct_FlareItem _array_element)) (.LocOpacityInfluence (Utilities|Struct|BreakStruct_FlareItem _array_element))))) _returnvalue_3)
        (else
          (bind _returnvalue_4 (Rendering|Material|CreateDynamicMaterialInstance 0 "None" :!class /Script/Engine.KismetMaterialLibrary))
          (Variables|/Game/LensFlareEff/Blueprints/FlareWidget.FlareWidget_C|SetCurrentMaterial (.FlareWidget (Utilities|Struct|BreakStruct_FlareItem (Utilities|Struct|MakeStruct_FlareItem (.Color (Utilities|Struct|BreakStruct_FlareItem _array_element)) _returnvalue (.FlareLocation (Utilities|Struct|BreakStruct_FlareItem _array_element)) (.IsMaterialAdditive (Utilities|Struct|BreakStruct_FlareItem _array_element)) (.FadeoutEdgeDistance (Utilities|Struct|BreakStruct_FlareItem _array_element)) (.ElementMaximumDistance (Utilities|Struct|BreakStruct_FlareItem _array_element)) (.FadeOut_EnableShrinking (Utilities|Struct|BreakStruct_FlareItem _array_element)) true (.FadeOut_FlareLocation (Utilities|Struct|BreakStruct_FlareItem _array_element)) (.Material (Utilities|Struct|BreakStruct_FlareItem _array_element)) (.ScreenPositionOffset (Utilities|Struct|BreakStruct_FlareItem _array_element)) (.GlobalSizeMultiplier (Utilities|Struct|BreakStruct_FlareItem _array_element)) (.InitialSpriteAngle (Utilities|Struct|BreakStruct_FlareItem _array_element)) (.ActiveRotationAmount (Utilities|Struct|BreakStruct_FlareItem _array_element)) (.EnableOrbitRotation (Utilities|Struct|BreakStruct_FlareItem _array_element)) (.EnablesLocationScaling (Utilities|Struct|BreakStruct_FlareItem _array_element)) (.LocationScalingInfluence (Utilities|Struct|BreakStruct_FlareItem _array_element)) (.LocationScalingCenterSize (Utilities|Struct|BreakStruct_FlareItem _array_element)) (.LocationScalingEdgeSize (Utilities|Struct|BreakStruct_FlareItem _array_element)) (.EnableLocationBasedOpacity (Utilities|Struct|BreakStruct_FlareItem _array_element)) (.LocOpacityCenterOpacity (Utilities|Struct|BreakStruct_FlareItem _array_element)) (.LocOpacityEdgeOpacity (Utilities|Struct|BreakStruct_FlareItem _array_element)) (.LocOpacityInfluence (Utilities|Struct|BreakStruct_FlareItem _array_element))))) _returnvalue_4))))
    (Default|Initialize (.FlareWidget (Utilities|Struct|BreakStruct_FlareItem (Utilities|Struct|MakeStruct_FlareItem (.Color (Utilities|Struct|BreakStruct_FlareItem _array_element)) _returnvalue (.FlareLocation (Utilities|Struct|BreakStruct_FlareItem _array_element)) (.IsMaterialAdditive (Utilities|Struct|BreakStruct_FlareItem _array_element)) (.FadeoutEdgeDistance (Utilities|Struct|BreakStruct_FlareItem _array_element)) (.ElementMaximumDistance (Utilities|Struct|BreakStruct_FlareItem _array_element)) (.FadeOut_EnableShrinking (Utilities|Struct|BreakStruct_FlareItem _array_element)) true (.FadeOut_FlareLocation (Utilities|Struct|BreakStruct_FlareItem _array_element)) (.Material (Utilities|Struct|BreakStruct_FlareItem _array_element)) (.ScreenPositionOffset (Utilities|Struct|BreakStruct_FlareItem _array_element)) (.GlobalSizeMultiplier (Utilities|Struct|BreakStruct_FlareItem _array_element)) (.InitialSpriteAngle (Utilities|Struct|BreakStruct_FlareItem _array_element)) (.ActiveRotationAmount (Utilities|Struct|BreakStruct_FlareItem _array_element)) (.EnableOrbitRotation (Utilities|Struct|BreakStruct_FlareItem _array_element)) (.EnablesLocationScaling (Utilities|Struct|BreakStruct_FlareItem _array_element)) (.LocationScalingInfluence (Utilities|Struct|BreakStruct_FlareItem _array_element)) (.LocationScalingCenterSize (Utilities|Struct|BreakStruct_FlareItem _array_element)) (.LocationScalingEdgeSize (Utilities|Struct|BreakStruct_FlareItem _array_element)) (.EnableLocationBasedOpacity (Utilities|Struct|BreakStruct_FlareItem _array_element)) (.LocOpacityCenterOpacity (Utilities|Struct|BreakStruct_FlareItem _array_element)) (.LocOpacityEdgeOpacity (Utilities|Struct|BreakStruct_FlareItem _array_element)) (.LocOpacityInfluence (Utilities|Struct|BreakStruct_FlareItem _array_element))))) (.FlareLocation (Utilities|Struct|BreakStruct_FlareItem (Utilities|Struct|MakeStruct_FlareItem (.Color (Utilities|Struct|BreakStruct_FlareItem _array_element)) _returnvalue (.FlareLocation (Utilities|Struct|BreakStruct_FlareItem _array_element)) (.IsMaterialAdditive (Utilities|Struct|BreakStruct_FlareItem _array_element)) (.FadeoutEdgeDistance (Utilities|Struct|BreakStruct_FlareItem _array_element)) (.ElementMaximumDistance (Utilities|Struct|BreakStruct_FlareItem _array_element)) (.FadeOut_EnableShrinking (Utilities|Struct|BreakStruct_FlareItem _array_element)) true (.FadeOut_FlareLocation (Utilities|Struct|BreakStruct_FlareItem _array_element)) (.Material (Utilities|Struct|BreakStruct_FlareItem _array_element)) (.ScreenPositionOffset (Utilities|Struct|BreakStruct_FlareItem _array_element)) (.GlobalSizeMultiplier (Utilities|Struct|BreakStruct_FlareItem _array_element)) (.InitialSpriteAngle (Utilities|Struct|BreakStruct_FlareItem _array_element)) (.ActiveRotationAmount (Utilities|Struct|BreakStruct_FlareItem _array_element)) (.EnableOrbitRotation (Utilities|Struct|BreakStruct_FlareItem _array_element)) (.EnablesLocationScaling (Utilities|Struct|BreakStruct_FlareItem _array_element)) (.LocationScalingInfluence (Utilities|Struct|BreakStruct_FlareItem _array_element)) (.LocationScalingCenterSize (Utilities|Struct|BreakStruct_FlareItem _array_element)) (.LocationScalingEdgeSize (Utilities|Struct|BreakStruct_FlareItem _array_element)) (.EnableLocationBasedOpacity (Utilities|Struct|BreakStruct_FlareItem _array_element)) (.LocOpacityCenterOpacity (Utilities|Struct|BreakStruct_FlareItem _array_element)) (.LocOpacityEdgeOpacity (Utilities|Struct|BreakStruct_FlareItem _array_element)) (.LocOpacityInfluence (Utilities|Struct|BreakStruct_FlareItem _array_element))))) (Transformation|GetWorldLocation (Variables|Default|GetDefaultSceneRoot)) (.X (Math|Vector2D|BreakVector2D (.FadeoutEdgeDistance (Utilities|Struct|BreakStruct_FlareItem (Utilities|Struct|MakeStruct_FlareItem (.Color (Utilities|Struct|BreakStruct_FlareItem _array_element)) _returnvalue (.FlareLocation (Utilities|Struct|BreakStruct_FlareItem _array_element)) (.IsMaterialAdditive (Utilities|Struct|BreakStruct_FlareItem _array_element)) (.FadeoutEdgeDistance (Utilities|Struct|BreakStruct_FlareItem _array_element)) (.ElementMaximumDistance (Utilities|Struct|BreakStruct_FlareItem _array_element)) (.FadeOut_EnableShrinking (Utilities|Struct|BreakStruct_FlareItem _array_element)) true (.FadeOut_FlareLocation (Utilities|Struct|BreakStruct_FlareItem _array_element)) (.Material (Utilities|Struct|BreakStruct_FlareItem _array_element)) (.ScreenPositionOffset (Utilities|Struct|BreakStruct_FlareItem _array_element)) (.GlobalSizeMultiplier (Utilities|Struct|BreakStruct_FlareItem _array_element)) (.InitialSpriteAngle (Utilities|Struct|BreakStruct_FlareItem _array_element)) (.ActiveRotationAmount (Utilities|Struct|BreakStruct_FlareItem _array_element)) (.EnableOrbitRotation (Utilities|Struct|BreakStruct_FlareItem _array_element)) (.EnablesLocationScaling (Utilities|Struct|BreakStruct_FlareItem _array_element)) (.LocationScalingInfluence (Utilities|Struct|BreakStruct_FlareItem _array_element)) (.LocationScalingCenterSize (Utilities|Struct|BreakStruct_FlareItem _array_element)) (.LocationScalingEdgeSize (Utilities|Struct|BreakStruct_FlareItem _array_element)) (.EnableLocationBasedOpacity (Utilities|Struct|BreakStruct_FlareItem _array_element)) (.LocOpacityCenterOpacity (Utilities|Struct|BreakStruct_FlareItem _array_element)) (.LocOpacityEdgeOpacity (Utilities|Struct|BreakStruct_FlareItem _array_element)) (.LocOpacityInfluence (Utilities|Struct|BreakStruct_FlareItem _array_element))))))) (.Y (Math|Vector2D|BreakVector2D (.FadeoutEdgeDistance (Utilities|Struct|BreakStruct_FlareItem (Utilities|Struct|MakeStruct_FlareItem (.Color (Utilities|Struct|BreakStruct_FlareItem _array_element)) _returnvalue (.FlareLocation (Utilities|Struct|BreakStruct_FlareItem _array_element)) (.IsMaterialAdditive (Utilities|Struct|BreakStruct_FlareItem _array_element)) (.FadeoutEdgeDistance (Utilities|Struct|BreakStruct_FlareItem _array_element)) (.ElementMaximumDistance (Utilities|Struct|BreakStruct_FlareItem _array_element)) (.FadeOut_EnableShrinking (Utilities|Struct|BreakStruct_FlareItem _array_element)) true (.FadeOut_FlareLocation (Utilities|Struct|BreakStruct_FlareItem _array_element)) (.Material (Utilities|Struct|BreakStruct_FlareItem _array_element)) (.ScreenPositionOffset (Utilities|Struct|BreakStruct_FlareItem _array_element)) (.GlobalSizeMultiplier (Utilities|Struct|BreakStruct_FlareItem _array_element)) (.InitialSpriteAngle (Utilities|Struct|BreakStruct_FlareItem _array_element)) (.ActiveRotationAmount (Utilities|Struct|BreakStruct_FlareItem _array_element)) (.EnableOrbitRotation (Utilities|Struct|BreakStruct_FlareItem _array_element)) (.EnablesLocationScaling (Utilities|Struct|BreakStruct_FlareItem _array_element)) (.LocationScalingInfluence (Utilities|Struct|BreakStruct_FlareItem _array_element)) (.LocationScalingCenterSize (Utilities|Struct|BreakStruct_FlareItem _array_element)) (.LocationScalingEdgeSize (Utilities|Struct|BreakStruct_FlareItem _array_element)) (.EnableLocationBasedOpacity (Utilities|Struct|BreakStruct_FlareItem _array_element)) (.LocOpacityCenterOpacity (Utilities|Struct|BreakStruct_FlareItem _array_element)) (.LocOpacityEdgeOpacity (Utilities|Struct|BreakStruct_FlareItem _array_element)) (.LocOpacityInfluence (Utilities|Struct|BreakStruct_FlareItem _array_element))))))) (.ElementMaximumDistance (Utilities|Struct|BreakStruct_FlareItem (Utilities|Struct|MakeStruct_FlareItem (.Color (Utilities|Struct|BreakStruct_FlareItem _array_element)) _returnvalue (.FlareLocation (Utilities|Struct|BreakStruct_FlareItem _array_element)) (.IsMaterialAdditive (Utilities|Struct|BreakStruct_FlareItem _array_element)) (.FadeoutEdgeDistance (Utilities|Struct|BreakStruct_FlareItem _array_element)) (.ElementMaximumDistance (Utilities|Struct|BreakStruct_FlareItem _array_element)) (.FadeOut_EnableShrinking (Utilities|Struct|BreakStruct_FlareItem _array_element)) true (.FadeOut_FlareLocation (Utilities|Struct|BreakStruct_FlareItem _array_element)) (.Material (Utilities|Struct|BreakStruct_FlareItem _array_element)) (.ScreenPositionOffset (Utilities|Struct|BreakStruct_FlareItem _array_element)) (.GlobalSizeMultiplier (Utilities|Struct|BreakStruct_FlareItem _array_element)) (.InitialSpriteAngle (Utilities|Struct|BreakStruct_FlareItem _array_element)) (.ActiveRotationAmount (Utilities|Struct|BreakStruct_FlareItem _array_element)) (.EnableOrbitRotation (Utilities|Struct|BreakStruct_FlareItem _array_element)) (.EnablesLocationScaling (Utilities|Struct|BreakStruct_FlareItem _array_element)) (.LocationScalingInfluence (Utilities|Struct|BreakStruct_FlareItem _array_element)) (.LocationScalingCenterSize (Utilities|Struct|BreakStruct_FlareItem _array_element)) (.LocationScalingEdgeSize (Utilities|Struct|BreakStruct_FlareItem _array_element)) (.EnableLocationBasedOpacity (Utilities|Struct|BreakStruct_FlareItem _array_element)) (.LocOpacityCenterOpacity (Utilities|Struct|BreakStruct_FlareItem _array_element)) (.LocOpacityEdgeOpacity (Utilities|Struct|BreakStruct_FlareItem _array_element)) (.LocOpacityInfluence (Utilities|Struct|BreakStruct_FlareItem _array_element))))) (.LocationScalingCenterSize (Utilities|Struct|BreakStruct_FlareItem (Utilities|Struct|MakeStruct_FlareItem (.Color (Utilities|Struct|BreakStruct_FlareItem _array_element)) _returnvalue (.FlareLocation (Utilities|Struct|BreakStruct_FlareItem _array_element)) (.IsMaterialAdditive (Utilities|Struct|BreakStruct_FlareItem _array_element)) (.FadeoutEdgeDistance (Utilities|Struct|BreakStruct_FlareItem _array_element)) (.ElementMaximumDistance (Utilities|Struct|BreakStruct_FlareItem _array_element)) (.FadeOut_EnableShrinking (Utilities|Struct|BreakStruct_FlareItem _array_element)) true (.FadeOut_FlareLocation (Utilities|Struct|BreakStruct_FlareItem _array_element)) (.Material (Utilities|Struct|BreakStruct_FlareItem _array_element)) (.ScreenPositionOffset (Utilities|Struct|BreakStruct_FlareItem _array_element)) (.GlobalSizeMultiplier (Utilities|Struct|BreakStruct_FlareItem _array_element)) (.InitialSpriteAngle (Utilities|Struct|BreakStruct_FlareItem _array_element)) (.ActiveRotationAmount (Utilities|Struct|BreakStruct_FlareItem _array_element)) (.EnableOrbitRotation (Utilities|Struct|BreakStruct_FlareItem _array_element)) (.EnablesLocationScaling (Utilities|Struct|BreakStruct_FlareItem _array_element)) (.LocationScalingInfluence (Utilities|Struct|BreakStruct_FlareItem _array_element)) (.LocationScalingCenterSize (Utilities|Struct|BreakStruct_FlareItem _array_element)) (.LocationScalingEdgeSize (Utilities|Struct|BreakStruct_FlareItem _array_element)) (.EnableLocationBasedOpacity (Utilities|Struct|BreakStruct_FlareItem _array_element)) (.LocOpacityCenterOpacity (Utilities|Struct|BreakStruct_FlareItem _array_element)) (.LocOpacityEdgeOpacity (Utilities|Struct|BreakStruct_FlareItem _array_element)) (.LocOpacityInfluence (Utilities|Struct|BreakStruct_FlareItem _array_element))))) (.LocationScalingEdgeSize (Utilities|Struct|BreakStruct_FlareItem (Utilities|Struct|MakeStruct_FlareItem (.Color (Utilities|Struct|BreakStruct_FlareItem _array_element)) _returnvalue (.FlareLocation (Utilities|Struct|BreakStruct_FlareItem _array_element)) (.IsMaterialAdditive (Utilities|Struct|BreakStruct_FlareItem _array_element)) (.FadeoutEdgeDistance (Utilities|Struct|BreakStruct_FlareItem _array_element)) (.ElementMaximumDistance (Utilities|Struct|BreakStruct_FlareItem _array_element)) (.FadeOut_EnableShrinking (Utilities|Struct|BreakStruct_FlareItem _array_element)) true (.FadeOut_FlareLocation (Utilities|Struct|BreakStruct_FlareItem _array_element)) (.Material (Utilities|Struct|BreakStruct_FlareItem _array_element)) (.ScreenPositionOffset (Utilities|Struct|BreakStruct_FlareItem _array_element)) (.GlobalSizeMultiplier (Utilities|Struct|BreakStruct_FlareItem _array_element)) (.InitialSpriteAngle (Utilities|Struct|BreakStruct_FlareItem _array_element)) (.ActiveRotationAmount (Utilities|Struct|BreakStruct_FlareItem _array_element)) (.EnableOrbitRotation (Utilities|Struct|BreakStruct_FlareItem _array_element)) (.EnablesLocationScaling (Utilities|Struct|BreakStruct_FlareItem _array_element)) (.LocationScalingInfluence (Utilities|Struct|BreakStruct_FlareItem _array_element)) (.LocationScalingCenterSize (Utilities|Struct|BreakStruct_FlareItem _array_element)) (.LocationScalingEdgeSize (Utilities|Struct|BreakStruct_FlareItem _array_element)) (.EnableLocationBasedOpacity (Utilities|Struct|BreakStruct_FlareItem _array_element)) (.LocOpacityCenterOpacity (Utilities|Struct|BreakStruct_FlareItem _array_element)) (.LocOpacityEdgeOpacity (Utilities|Struct|BreakStruct_FlareItem _array_element)) (.LocOpacityInfluence (Utilities|Struct|BreakStruct_FlareItem _array_element))))) (.LocationScalingInfluence (Utilities|Struct|BreakStruct_FlareItem (Utilities|Struct|MakeStruct_FlareItem (.Color (Utilities|Struct|BreakStruct_FlareItem _array_element)) _returnvalue (.FlareLocation (Utilities|Struct|BreakStruct_FlareItem _array_element)) (.IsMaterialAdditive (Utilities|Struct|BreakStruct_FlareItem _array_element)) (.FadeoutEdgeDistance (Utilities|Struct|BreakStruct_FlareItem _array_element)) (.ElementMaximumDistance (Utilities|Struct|BreakStruct_FlareItem _array_element)) (.FadeOut_EnableShrinking (Utilities|Struct|BreakStruct_FlareItem _array_element)) true (.FadeOut_FlareLocation (Utilities|Struct|BreakStruct_FlareItem _array_element)) (.Material (Utilities|Struct|BreakStruct_FlareItem _array_element)) (.ScreenPositionOffset (Utilities|Struct|BreakStruct_FlareItem _array_element)) (.GlobalSizeMultiplier (Utilities|Struct|BreakStruct_FlareItem _array_element)) (.InitialSpriteAngle (Utilities|Struct|BreakStruct_FlareItem _array_element)) (.ActiveRotationAmount (Utilities|Struct|BreakStruct_FlareItem _array_element)) (.EnableOrbitRotation (Utilities|Struct|BreakStruct_FlareItem _array_element)) (.EnablesLocationScaling (Utilities|Struct|BreakStruct_FlareItem _array_element)) (.LocationScalingInfluence (Utilities|Struct|BreakStruct_FlareItem _array_element)) (.LocationScalingCenterSize (Utilities|Struct|BreakStruct_FlareItem _array_element)) (.LocationScalingEdgeSize (Utilities|Struct|BreakStruct_FlareItem _array_element)) (.EnableLocationBasedOpacity (Utilities|Struct|BreakStruct_FlareItem _array_element)) (.LocOpacityCenterOpacity (Utilities|Struct|BreakStruct_FlareItem _array_element)) (.LocOpacityEdgeOpacity (Utilities|Struct|BreakStruct_FlareItem _array_element)) (.LocOpacityInfluence (Utilities|Struct|BreakStruct_FlareItem _array_element))))) (.EnablesLocationScaling (Utilities|Struct|BreakStruct_FlareItem (Utilities|Struct|MakeStruct_FlareItem (.Color (Utilities|Struct|BreakStruct_FlareItem _array_element)) _returnvalue (.FlareLocation (Utilities|Struct|BreakStruct_FlareItem _array_element)) (.IsMaterialAdditive (Utilities|Struct|BreakStruct_FlareItem _array_element)) (.FadeoutEdgeDistance (Utilities|Struct|BreakStruct_FlareItem _array_element)) (.ElementMaximumDistance (Utilities|Struct|BreakStruct_FlareItem _array_element)) (.FadeOut_EnableShrinking (Utilities|Struct|BreakStruct_FlareItem _array_element)) true (.FadeOut_FlareLocation (Utilities|Struct|BreakStruct_FlareItem _array_element)) (.Material (Utilities|Struct|BreakStruct_FlareItem _array_element)) (.ScreenPositionOffset (Utilities|Struct|BreakStruct_FlareItem _array_element)) (.GlobalSizeMultiplier (Utilities|Struct|BreakStruct_FlareItem _array_element)) (.InitialSpriteAngle (Utilities|Struct|BreakStruct_FlareItem _array_element)) (.ActiveRotationAmount (Utilities|Struct|BreakStruct_FlareItem _array_element)) (.EnableOrbitRotation (Utilities|Struct|BreakStruct_FlareItem _array_element)) (.EnablesLocationScaling (Utilities|Struct|BreakStruct_FlareItem _array_element)) (.LocationScalingInfluence (Utilities|Struct|BreakStruct_FlareItem _array_element)) (.LocationScalingCenterSize (Utilities|Struct|BreakStruct_FlareItem _array_element)) (.LocationScalingEdgeSize (Utilities|Struct|BreakStruct_FlareItem _array_element)) (.EnableLocationBasedOpacity (Utilities|Struct|BreakStruct_FlareItem _array_element)) (.LocOpacityCenterOpacity (Utilities|Struct|BreakStruct_FlareItem _array_element)) (.LocOpacityEdgeOpacity (Utilities|Struct|BreakStruct_FlareItem _array_element)) (.LocOpacityInfluence (Utilities|Struct|BreakStruct_FlareItem _array_element))))) (.ScreenPositionOffset (Utilities|Struct|BreakStruct_FlareItem (Utilities|Struct|MakeStruct_FlareItem (.Color (Utilities|Struct|BreakStruct_FlareItem _array_element)) _returnvalue (.FlareLocation (Utilities|Struct|BreakStruct_FlareItem _array_element)) (.IsMaterialAdditive (Utilities|Struct|BreakStruct_FlareItem _array_element)) (.FadeoutEdgeDistance (Utilities|Struct|BreakStruct_FlareItem _array_element)) (.ElementMaximumDistance (Utilities|Struct|BreakStruct_FlareItem _array_element)) (.FadeOut_EnableShrinking (Utilities|Struct|BreakStruct_FlareItem _array_element)) true (.FadeOut_FlareLocation (Utilities|Struct|BreakStruct_FlareItem _array_element)) (.Material (Utilities|Struct|BreakStruct_FlareItem _array_element)) (.ScreenPositionOffset (Utilities|Struct|BreakStruct_FlareItem _array_element)) (.GlobalSizeMultiplier (Utilities|Struct|BreakStruct_FlareItem _array_element)) (.InitialSpriteAngle (Utilities|Struct|BreakStruct_FlareItem _array_element)) (.ActiveRotationAmount (Utilities|Struct|BreakStruct_FlareItem _array_element)) (.EnableOrbitRotation (Utilities|Struct|BreakStruct_FlareItem _array_element)) (.EnablesLocationScaling (Utilities|Struct|BreakStruct_FlareItem _array_element)) (.LocationScalingInfluence (Utilities|Struct|BreakStruct_FlareItem _array_element)) (.LocationScalingCenterSize (Utilities|Struct|BreakStruct_FlareItem _array_element)) (.LocationScalingEdgeSize (Utilities|Struct|BreakStruct_FlareItem _array_element)) (.EnableLocationBasedOpacity (Utilities|Struct|BreakStruct_FlareItem _array_element)) (.LocOpacityCenterOpacity (Utilities|Struct|BreakStruct_FlareItem _array_element)) (.LocOpacityEdgeOpacity (Utilities|Struct|BreakStruct_FlareItem _array_element)) (.LocOpacityInfluence (Utilities|Struct|BreakStruct_FlareItem _array_element))))) (.EnableOrbitRotation (Utilities|Struct|BreakStruct_FlareItem (Utilities|Struct|MakeStruct_FlareItem (.Color (Utilities|Struct|BreakStruct_FlareItem _array_element)) _returnvalue (.FlareLocation (Utilities|Struct|BreakStruct_FlareItem _array_element)) (.IsMaterialAdditive (Utilities|Struct|BreakStruct_FlareItem _array_element)) (.FadeoutEdgeDistance (Utilities|Struct|BreakStruct_FlareItem _array_element)) (.ElementMaximumDistance (Utilities|Struct|BreakStruct_FlareItem _array_element)) (.FadeOut_EnableShrinking (Utilities|Struct|BreakStruct_FlareItem _array_element)) true (.FadeOut_FlareLocation (Utilities|Struct|BreakStruct_FlareItem _array_element)) (.Material (Utilities|Struct|BreakStruct_FlareItem _array_element)) (.ScreenPositionOffset (Utilities|Struct|BreakStruct_FlareItem _array_element)) (.GlobalSizeMultiplier (Utilities|Struct|BreakStruct_FlareItem _array_element)) (.InitialSpriteAngle (Utilities|Struct|BreakStruct_FlareItem _array_element)) (.ActiveRotationAmount (Utilities|Struct|BreakStruct_FlareItem _array_element)) (.EnableOrbitRotation (Utilities|Struct|BreakStruct_FlareItem _array_element)) (.EnablesLocationScaling (Utilities|Struct|BreakStruct_FlareItem _array_element)) (.LocationScalingInfluence (Utilities|Struct|BreakStruct_FlareItem _array_element)) (.LocationScalingCenterSize (Utilities|Struct|BreakStruct_FlareItem _array_element)) (.LocationScalingEdgeSize (Utilities|Struct|BreakStruct_FlareItem _array_element)) (.EnableLocationBasedOpacity (Utilities|Struct|BreakStruct_FlareItem _array_element)) (.LocOpacityCenterOpacity (Utilities|Struct|BreakStruct_FlareItem _array_element)) (.LocOpacityEdgeOpacity (Utilities|Struct|BreakStruct_FlareItem _array_element)) (.LocOpacityInfluence (Utilities|Struct|BreakStruct_FlareItem _array_element))))) (.InitialSpriteAngle (Utilities|Struct|BreakStruct_FlareItem (Utilities|Struct|MakeStruct_FlareItem (.Color (Utilities|Struct|BreakStruct_FlareItem _array_element)) _returnvalue (.FlareLocation (Utilities|Struct|BreakStruct_FlareItem _array_element)) (.IsMaterialAdditive (Utilities|Struct|BreakStruct_FlareItem _array_element)) (.FadeoutEdgeDistance (Utilities|Struct|BreakStruct_FlareItem _array_element)) (.ElementMaximumDistance (Utilities|Struct|BreakStruct_FlareItem _array_element)) (.FadeOut_EnableShrinking (Utilities|Struct|BreakStruct_FlareItem _array_element)) true (.FadeOut_FlareLocation (Utilities|Struct|BreakStruct_FlareItem _array_element)) (.Material (Utilities|Struct|BreakStruct_FlareItem _array_element)) (.ScreenPositionOffset (Utilities|Struct|BreakStruct_FlareItem _array_element)) (.GlobalSizeMultiplier (Utilities|Struct|BreakStruct_FlareItem _array_element)) (.InitialSpriteAngle (Utilities|Struct|BreakStruct_FlareItem _array_element)) (.ActiveRotationAmount (Utilities|Struct|BreakStruct_FlareItem _array_element)) (.EnableOrbitRotation (Utilities|Struct|BreakStruct_FlareItem _array_element)) (.EnablesLocationScaling (Utilities|Struct|BreakStruct_FlareItem _array_element)) (.LocationScalingInfluence (Utilities|Struct|BreakStruct_FlareItem _array_element)) (.LocationScalingCenterSize (Utilities|Struct|BreakStruct_FlareItem _array_element)) (.LocationScalingEdgeSize (Utilities|Struct|BreakStruct_FlareItem _array_element)) (.EnableLocationBasedOpacity (Utilities|Struct|BreakStruct_FlareItem _array_element)) (.LocOpacityCenterOpacity (Utilities|Struct|BreakStruct_FlareItem _array_element)) (.LocOpacityEdgeOpacity (Utilities|Struct|BreakStruct_FlareItem _array_element)) (.LocOpacityInfluence (Utilities|Struct|BreakStruct_FlareItem _array_element))))) (.GlobalSizeMultiplier (Utilities|Struct|BreakStruct_FlareItem (Utilities|Struct|MakeStruct_FlareItem (.Color (Utilities|Struct|BreakStruct_FlareItem _array_element)) _returnvalue (.FlareLocation (Utilities|Struct|BreakStruct_FlareItem _array_element)) (.IsMaterialAdditive (Utilities|Struct|BreakStruct_FlareItem _array_element)) (.FadeoutEdgeDistance (Utilities|Struct|BreakStruct_FlareItem _array_element)) (.ElementMaximumDistance (Utilities|Struct|BreakStruct_FlareItem _array_element)) (.FadeOut_EnableShrinking (Utilities|Struct|BreakStruct_FlareItem _array_element)) true (.FadeOut_FlareLocation (Utilities|Struct|BreakStruct_FlareItem _array_element)) (.Material (Utilities|Struct|BreakStruct_FlareItem _array_element)) (.ScreenPositionOffset (Utilities|Struct|BreakStruct_FlareItem _array_element)) (.GlobalSizeMultiplier (Utilities|Struct|BreakStruct_FlareItem _array_element)) (.InitialSpriteAngle (Utilities|Struct|BreakStruct_FlareItem _array_element)) (.ActiveRotationAmount (Utilities|Struct|BreakStruct_FlareItem _array_element)) (.EnableOrbitRotation (Utilities|Struct|BreakStruct_FlareItem _array_element)) (.EnablesLocationScaling (Utilities|Struct|BreakStruct_FlareItem _array_element)) (.LocationScalingInfluence (Utilities|Struct|BreakStruct_FlareItem _array_element)) (.LocationScalingCenterSize (Utilities|Struct|BreakStruct_FlareItem _array_element)) (.LocationScalingEdgeSize (Utilities|Struct|BreakStruct_FlareItem _array_element)) (.EnableLocationBasedOpacity (Utilities|Struct|BreakStruct_FlareItem _array_element)) (.LocOpacityCenterOpacity (Utilities|Struct|BreakStruct_FlareItem _array_element)) (.LocOpacityEdgeOpacity (Utilities|Struct|BreakStruct_FlareItem _array_element)) (.LocOpacityInfluence (Utilities|Struct|BreakStruct_FlareItem _array_element))))) (.FadeOut_EnableShrinking (Utilities|Struct|BreakStruct_FlareItem (Utilities|Struct|MakeStruct_FlareItem (.Color (Utilities|Struct|BreakStruct_FlareItem _array_element)) _returnvalue (.FlareLocation (Utilities|Struct|BreakStruct_FlareItem _array_element)) (.IsMaterialAdditive (Utilities|Struct|BreakStruct_FlareItem _array_element)) (.FadeoutEdgeDistance (Utilities|Struct|BreakStruct_FlareItem _array_element)) (.ElementMaximumDistance (Utilities|Struct|BreakStruct_FlareItem _array_element)) (.FadeOut_EnableShrinking (Utilities|Struct|BreakStruct_FlareItem _array_element)) true (.FadeOut_FlareLocation (Utilities|Struct|BreakStruct_FlareItem _array_element)) (.Material (Utilities|Struct|BreakStruct_FlareItem _array_element)) (.ScreenPositionOffset (Utilities|Struct|BreakStruct_FlareItem _array_element)) (.GlobalSizeMultiplier (Utilities|Struct|BreakStruct_FlareItem _array_element)) (.InitialSpriteAngle (Utilities|Struct|BreakStruct_FlareItem _array_element)) (.ActiveRotationAmount (Utilities|Struct|BreakStruct_FlareItem _array_element)) (.EnableOrbitRotation (Utilities|Struct|BreakStruct_FlareItem _array_element)) (.EnablesLocationScaling (Utilities|Struct|BreakStruct_FlareItem _array_element)) (.LocationScalingInfluence (Utilities|Struct|BreakStruct_FlareItem _array_element)) (.LocationScalingCenterSize (Utilities|Struct|BreakStruct_FlareItem _array_element)) (.LocationScalingEdgeSize (Utilities|Struct|BreakStruct_FlareItem _array_element)) (.EnableLocationBasedOpacity (Utilities|Struct|BreakStruct_FlareItem _array_element)) (.LocOpacityCenterOpacity (Utilities|Struct|BreakStruct_FlareItem _array_element)) (.LocOpacityEdgeOpacity (Utilities|Struct|BreakStruct_FlareItem _array_element)) (.LocOpacityInfluence (Utilities|Struct|BreakStruct_FlareItem _array_element))))) (Variables|Default|GetFDopacity) (.FadeOut_FlareLocation (Utilities|Struct|BreakStruct_FlareItem (Utilities|Struct|MakeStruct_FlareItem (.Color (Utilities|Struct|BreakStruct_FlareItem _array_element)) _returnvalue (.FlareLocation (Utilities|Struct|BreakStruct_FlareItem _array_element)) (.IsMaterialAdditive (Utilities|Struct|BreakStruct_FlareItem _array_element)) (.FadeoutEdgeDistance (Utilities|Struct|BreakStruct_FlareItem _array_element)) (.ElementMaximumDistance (Utilities|Struct|BreakStruct_FlareItem _array_element)) (.FadeOut_EnableShrinking (Utilities|Struct|BreakStruct_FlareItem _array_element)) true (.FadeOut_FlareLocation (Utilities|Struct|BreakStruct_FlareItem _array_element)) (.Material (Utilities|Struct|BreakStruct_FlareItem _array_element)) (.ScreenPositionOffset (Utilities|Struct|BreakStruct_FlareItem _array_element)) (.GlobalSizeMultiplier (Utilities|Struct|BreakStruct_FlareItem _array_element)) (.InitialSpriteAngle (Utilities|Struct|BreakStruct_FlareItem _array_element)) (.ActiveRotationAmount (Utilities|Struct|BreakStruct_FlareItem _array_element)) (.EnableOrbitRotation (Utilities|Struct|BreakStruct_FlareItem _array_element)) (.EnablesLocationScaling (Utilities|Struct|BreakStruct_FlareItem _array_element)) (.LocationScalingInfluence (Utilities|Struct|BreakStruct_FlareItem _array_element)) (.LocationScalingCenterSize (Utilities|Struct|BreakStruct_FlareItem _array_element)) (.LocationScalingEdgeSize (Utilities|Struct|BreakStruct_FlareItem _array_element)) (.EnableLocationBasedOpacity (Utilities|Struct|BreakStruct_FlareItem _array_element)) (.LocOpacityCenterOpacity (Utilities|Struct|BreakStruct_FlareItem _array_element)) (.LocOpacityEdgeOpacity (Utilities|Struct|BreakStruct_FlareItem _array_element)) (.LocOpacityInfluence (Utilities|Struct|BreakStruct_FlareItem _array_element))))) (.EnableLocationBasedOpacity (Utilities|Struct|BreakStruct_FlareItem (Utilities|Struct|MakeStruct_FlareItem (.Color (Utilities|Struct|BreakStruct_FlareItem _array_element)) _returnvalue (.FlareLocation (Utilities|Struct|BreakStruct_FlareItem _array_element)) (.IsMaterialAdditive (Utilities|Struct|BreakStruct_FlareItem _array_element)) (.FadeoutEdgeDistance (Utilities|Struct|BreakStruct_FlareItem _array_element)) (.ElementMaximumDistance (Utilities|Struct|BreakStruct_FlareItem _array_element)) (.FadeOut_EnableShrinking (Utilities|Struct|BreakStruct_FlareItem _array_element)) true (.FadeOut_FlareLocation (Utilities|Struct|BreakStruct_FlareItem _array_element)) (.Material (Utilities|Struct|BreakStruct_FlareItem _array_element)) (.ScreenPositionOffset (Utilities|Struct|BreakStruct_FlareItem _array_element)) (.GlobalSizeMultiplier (Utilities|Struct|BreakStruct_FlareItem _array_element)) (.InitialSpriteAngle (Utilities|Struct|BreakStruct_FlareItem _array_element)) (.ActiveRotationAmount (Utilities|Struct|BreakStruct_FlareItem _array_element)) (.EnableOrbitRotation (Utilities|Struct|BreakStruct_FlareItem _array_element)) (.EnablesLocationScaling (Utilities|Struct|BreakStruct_FlareItem _array_element)) (.LocationScalingInfluence (Utilities|Struct|BreakStruct_FlareItem _array_element)) (.LocationScalingCenterSize (Utilities|Struct|BreakStruct_FlareItem _array_element)) (.LocationScalingEdgeSize (Utilities|Struct|BreakStruct_FlareItem _array_element)) (.EnableLocationBasedOpacity (Utilities|Struct|BreakStruct_FlareItem _array_element)) (.LocOpacityCenterOpacity (Utilities|Struct|BreakStruct_FlareItem _array_element)) (.LocOpacityEdgeOpacity (Utilities|Struct|BreakStruct_FlareItem _array_element)) (.LocOpacityInfluence (Utilities|Struct|BreakStruct_FlareItem _array_element))))) (.LocOpacityCenterOpacity (Utilities|Struct|BreakStruct_FlareItem (Utilities|Struct|MakeStruct_FlareItem (.Color (Utilities|Struct|BreakStruct_FlareItem _array_element)) _returnvalue (.FlareLocation (Utilities|Struct|BreakStruct_FlareItem _array_element)) (.IsMaterialAdditive (Utilities|Struct|BreakStruct_FlareItem _array_element)) (.FadeoutEdgeDistance (Utilities|Struct|BreakStruct_FlareItem _array_element)) (.ElementMaximumDistance (Utilities|Struct|BreakStruct_FlareItem _array_element)) (.FadeOut_EnableShrinking (Utilities|Struct|BreakStruct_FlareItem _array_element)) true (.FadeOut_FlareLocation (Utilities|Struct|BreakStruct_FlareItem _array_element)) (.Material (Utilities|Struct|BreakStruct_FlareItem _array_element)) (.ScreenPositionOffset (Utilities|Struct|BreakStruct_FlareItem _array_element)) (.GlobalSizeMultiplier (Utilities|Struct|BreakStruct_FlareItem _array_element)) (.InitialSpriteAngle (Utilities|Struct|BreakStruct_FlareItem _array_element)) (.ActiveRotationAmount (Utilities|Struct|BreakStruct_FlareItem _array_element)) (.EnableOrbitRotation (Utilities|Struct|BreakStruct_FlareItem _array_element)) (.EnablesLocationScaling (Utilities|Struct|BreakStruct_FlareItem _array_element)) (.LocationScalingInfluence (Utilities|Struct|BreakStruct_FlareItem _array_element)) (.LocationScalingCenterSize (Utilities|Struct|BreakStruct_FlareItem _array_element)) (.LocationScalingEdgeSize (Utilities|Struct|BreakStruct_FlareItem _array_element)) (.EnableLocationBasedOpacity (Utilities|Struct|BreakStruct_FlareItem _array_element)) (.LocOpacityCenterOpacity (Utilities|Struct|BreakStruct_FlareItem _array_element)) (.LocOpacityEdgeOpacity (Utilities|Struct|BreakStruct_FlareItem _array_element)) (.LocOpacityInfluence (Utilities|Struct|BreakStruct_FlareItem _array_element))))) (.LocOpacityEdgeOpacity (Utilities|Struct|BreakStruct_FlareItem (Utilities|Struct|MakeStruct_FlareItem (.Color (Utilities|Struct|BreakStruct_FlareItem _array_element)) _returnvalue (.FlareLocation (Utilities|Struct|BreakStruct_FlareItem _array_element)) (.IsMaterialAdditive (Utilities|Struct|BreakStruct_FlareItem _array_element)) (.FadeoutEdgeDistance (Utilities|Struct|BreakStruct_FlareItem _array_element)) (.ElementMaximumDistance (Utilities|Struct|BreakStruct_FlareItem _array_element)) (.FadeOut_EnableShrinking (Utilities|Struct|BreakStruct_FlareItem _array_element)) true (.FadeOut_FlareLocation (Utilities|Struct|BreakStruct_FlareItem _array_element)) (.Material (Utilities|Struct|BreakStruct_FlareItem _array_element)) (.ScreenPositionOffset (Utilities|Struct|BreakStruct_FlareItem _array_element)) (.GlobalSizeMultiplier (Utilities|Struct|BreakStruct_FlareItem _array_element)) (.InitialSpriteAngle (Utilities|Struct|BreakStruct_FlareItem _array_element)) (.ActiveRotationAmount (Utilities|Struct|BreakStruct_FlareItem _array_element)) (.EnableOrbitRotation (Utilities|Struct|BreakStruct_FlareItem _array_element)) (.EnablesLocationScaling (Utilities|Struct|BreakStruct_FlareItem _array_element)) (.LocationScalingInfluence (Utilities|Struct|BreakStruct_FlareItem _array_element)) (.LocationScalingCenterSize (Utilities|Struct|BreakStruct_FlareItem _array_element)) (.LocationScalingEdgeSize (Utilities|Struct|BreakStruct_FlareItem _array_element)) (.EnableLocationBasedOpacity (Utilities|Struct|BreakStruct_FlareItem _array_element)) (.LocOpacityCenterOpacity (Utilities|Struct|BreakStruct_FlareItem _array_element)) (.LocOpacityEdgeOpacity (Utilities|Struct|BreakStruct_FlareItem _array_element)) (.LocOpacityInfluence (Utilities|Struct|BreakStruct_FlareItem _array_element))))) (.LocOpacityInfluence (Utilities|Struct|BreakStruct_FlareItem (Utilities|Struct|MakeStruct_FlareItem (.Color (Utilities|Struct|BreakStruct_FlareItem _array_element)) _returnvalue (.FlareLocation (Utilities|Struct|BreakStruct_FlareItem _array_element)) (.IsMaterialAdditive (Utilities|Struct|BreakStruct_FlareItem _array_element)) (.FadeoutEdgeDistance (Utilities|Struct|BreakStruct_FlareItem _array_element)) (.ElementMaximumDistance (Utilities|Struct|BreakStruct_FlareItem _array_element)) (.FadeOut_EnableShrinking (Utilities|Struct|BreakStruct_FlareItem _array_element)) true (.FadeOut_FlareLocation (Utilities|Struct|BreakStruct_FlareItem _array_element)) (.Material (Utilities|Struct|BreakStruct_FlareItem _array_element)) (.ScreenPositionOffset (Utilities|Struct|BreakStruct_FlareItem _array_element)) (.GlobalSizeMultiplier (Utilities|Struct|BreakStruct_FlareItem _array_element)) (.InitialSpriteAngle (Utilities|Struct|BreakStruct_FlareItem _array_element)) (.ActiveRotationAmount (Utilities|Struct|BreakStruct_FlareItem _array_element)) (.EnableOrbitRotation (Utilities|Struct|BreakStruct_FlareItem _array_element)) (.EnablesLocationScaling (Utilities|Struct|BreakStruct_FlareItem _array_element)) (.LocationScalingInfluence (Utilities|Struct|BreakStruct_FlareItem _array_element)) (.LocationScalingCenterSize (Utilities|Struct|BreakStruct_FlareItem _array_element)) (.LocationScalingEdgeSize (Utilities|Struct|BreakStruct_FlareItem _array_element)) (.EnableLocationBasedOpacity (Utilities|Struct|BreakStruct_FlareItem _array_element)) (.LocOpacityCenterOpacity (Utilities|Struct|BreakStruct_FlareItem _array_element)) (.LocOpacityEdgeOpacity (Utilities|Struct|BreakStruct_FlareItem _array_element)) (.LocOpacityInfluence (Utilities|Struct|BreakStruct_FlareItem _array_element))))) (.ActiveRotationAmount (Utilities|Struct|BreakStruct_FlareItem (Utilities|Struct|MakeStruct_FlareItem (.Color (Utilities|Struct|BreakStruct_FlareItem _array_element)) _returnvalue (.FlareLocation (Utilities|Struct|BreakStruct_FlareItem _array_element)) (.IsMaterialAdditive (Utilities|Struct|BreakStruct_FlareItem _array_element)) (.FadeoutEdgeDistance (Utilities|Struct|BreakStruct_FlareItem _array_element)) (.ElementMaximumDistance (Utilities|Struct|BreakStruct_FlareItem _array_element)) (.FadeOut_EnableShrinking (Utilities|Struct|BreakStruct_FlareItem _array_element)) true (.FadeOut_FlareLocation (Utilities|Struct|BreakStruct_FlareItem _array_element)) (.Material (Utilities|Struct|BreakStruct_FlareItem _array_element)) (.ScreenPositionOffset (Utilities|Struct|BreakStruct_FlareItem _array_element)) (.GlobalSizeMultiplier (Utilities|Struct|BreakStruct_FlareItem _array_element)) (.InitialSpriteAngle (Utilities|Struct|BreakStruct_FlareItem _array_element)) (.ActiveRotationAmount (Utilities|Struct|BreakStruct_FlareItem _array_element)) (.EnableOrbitRotation (Utilities|Struct|BreakStruct_FlareItem _array_element)) (.EnablesLocationScaling (Utilities|Struct|BreakStruct_FlareItem _array_element)) (.LocationScalingInfluence (Utilities|Struct|BreakStruct_FlareItem _array_element)) (.LocationScalingCenterSize (Utilities|Struct|BreakStruct_FlareItem _array_element)) (.LocationScalingEdgeSize (Utilities|Struct|BreakStruct_FlareItem _array_element)) (.EnableLocationBasedOpacity (Utilities|Struct|BreakStruct_FlareItem _array_element)) (.LocOpacityCenterOpacity (Utilities|Struct|BreakStruct_FlareItem _array_element)) (.LocOpacityEdgeOpacity (Utilities|Struct|BreakStruct_FlareItem _array_element)) (.LocOpacityInfluence (Utilities|Struct|BreakStruct_FlareItem _array_element))))) (.SpecifiedColor (Utilities|Struct|BreakSlateColor (.Color (Utilities|Struct|BreakStruct_FlareItem (Utilities|Struct|MakeStruct_FlareItem (.Color (Utilities|Struct|BreakStruct_FlareItem _array_element)) _returnvalue (.FlareLocation (Utilities|Struct|BreakStruct_FlareItem _array_element)) (.IsMaterialAdditive (Utilities|Struct|BreakStruct_FlareItem _array_element)) (.FadeoutEdgeDistance (Utilities|Struct|BreakStruct_FlareItem _array_element)) (.ElementMaximumDistance (Utilities|Struct|BreakStruct_FlareItem _array_element)) (.FadeOut_EnableShrinking (Utilities|Struct|BreakStruct_FlareItem _array_element)) true (.FadeOut_FlareLocation (Utilities|Struct|BreakStruct_FlareItem _array_element)) (.Material (Utilities|Struct|BreakStruct_FlareItem _array_element)) (.ScreenPositionOffset (Utilities|Struct|BreakStruct_FlareItem _array_element)) (.GlobalSizeMultiplier (Utilities|Struct|BreakStruct_FlareItem _array_element)) (.InitialSpriteAngle (Utilities|Struct|BreakStruct_FlareItem _array_element)) (.ActiveRotationAmount (Utilities|Struct|BreakStruct_FlareItem _array_element)) (.EnableOrbitRotation (Utilities|Struct|BreakStruct_FlareItem _array_element)) (.EnablesLocationScaling (Utilities|Struct|BreakStruct_FlareItem _array_element)) (.LocationScalingInfluence (Utilities|Struct|BreakStruct_FlareItem _array_element)) (.LocationScalingCenterSize (Utilities|Struct|BreakStruct_FlareItem _array_element)) (.LocationScalingEdgeSize (Utilities|Struct|BreakStruct_FlareItem _array_element)) (.EnableLocationBasedOpacity (Utilities|Struct|BreakStruct_FlareItem _array_element)) (.LocOpacityCenterOpacity (Utilities|Struct|BreakStruct_FlareItem _array_element)) (.LocOpacityEdgeOpacity (Utilities|Struct|BreakStruct_FlareItem _array_element)) (.LocOpacityInfluence (Utilities|Struct|BreakStruct_FlareItem _array_element))))))) (.IsMaterialAdditive (Utilities|Struct|BreakStruct_FlareItem (Utilities|Struct|MakeStruct_FlareItem (.Color (Utilities|Struct|BreakStruct_FlareItem _array_element)) _returnvalue (.FlareLocation (Utilities|Struct|BreakStruct_FlareItem _array_element)) (.IsMaterialAdditive (Utilities|Struct|BreakStruct_FlareItem _array_element)) (.FadeoutEdgeDistance (Utilities|Struct|BreakStruct_FlareItem _array_element)) (.ElementMaximumDistance (Utilities|Struct|BreakStruct_FlareItem _array_element)) (.FadeOut_EnableShrinking (Utilities|Struct|BreakStruct_FlareItem _array_element)) true (.FadeOut_FlareLocation (Utilities|Struct|BreakStruct_FlareItem _array_element)) (.Material (Utilities|Struct|BreakStruct_FlareItem _array_element)) (.ScreenPositionOffset (Utilities|Struct|BreakStruct_FlareItem _array_element)) (.GlobalSizeMultiplier (Utilities|Struct|BreakStruct_FlareItem _array_element)) (.InitialSpriteAngle (Utilities|Struct|BreakStruct_FlareItem _array_element)) (.ActiveRotationAmount (Utilities|Struct|BreakStruct_FlareItem _array_element)) (.EnableOrbitRotation (Utilities|Struct|BreakStruct_FlareItem _array_element)) (.EnablesLocationScaling (Utilities|Struct|BreakStruct_FlareItem _array_element)) (.LocationScalingInfluence (Utilities|Struct|BreakStruct_FlareItem _array_element)) (.LocationScalingCenterSize (Utilities|Struct|BreakStruct_FlareItem _array_element)) (.LocationScalingEdgeSize (Utilities|Struct|BreakStruct_FlareItem _array_element)) (.EnableLocationBasedOpacity (Utilities|Struct|BreakStruct_FlareItem _array_element)) (.LocOpacityCenterOpacity (Utilities|Struct|BreakStruct_FlareItem _array_element)) (.LocOpacityEdgeOpacity (Utilities|Struct|BreakStruct_FlareItem _array_element)) (.LocOpacityInfluence (Utilities|Struct|BreakStruct_FlareItem _array_element))))))
    (Utilities|Array|Add (Variables|Default|GetWidgetList) (.FlareWidget (Utilities|Struct|BreakStruct_FlareItem (Utilities|Struct|MakeStruct_FlareItem (.Color (Utilities|Struct|BreakStruct_FlareItem _array_element)) _returnvalue (.FlareLocation (Utilities|Struct|BreakStruct_FlareItem _array_element)) (.IsMaterialAdditive (Utilities|Struct|BreakStruct_FlareItem _array_element)) (.FadeoutEdgeDistance (Utilities|Struct|BreakStruct_FlareItem _array_element)) (.ElementMaximumDistance (Utilities|Struct|BreakStruct_FlareItem _array_element)) (.FadeOut_EnableShrinking (Utilities|Struct|BreakStruct_FlareItem _array_element)) true (.FadeOut_FlareLocation (Utilities|Struct|BreakStruct_FlareItem _array_element)) (.Material (Utilities|Struct|BreakStruct_FlareItem _array_element)) (.ScreenPositionOffset (Utilities|Struct|BreakStruct_FlareItem _array_element)) (.GlobalSizeMultiplier (Utilities|Struct|BreakStruct_FlareItem _array_element)) (.InitialSpriteAngle (Utilities|Struct|BreakStruct_FlareItem _array_element)) (.ActiveRotationAmount (Utilities|Struct|BreakStruct_FlareItem _array_element)) (.EnableOrbitRotation (Utilities|Struct|BreakStruct_FlareItem _array_element)) (.EnablesLocationScaling (Utilities|Struct|BreakStruct_FlareItem _array_element)) (.LocationScalingInfluence (Utilities|Struct|BreakStruct_FlareItem _array_element)) (.LocationScalingCenterSize (Utilities|Struct|BreakStruct_FlareItem _array_element)) (.LocationScalingEdgeSize (Utilities|Struct|BreakStruct_FlareItem _array_element)) (.EnableLocationBasedOpacity (Utilities|Struct|BreakStruct_FlareItem _array_element)) (.LocOpacityCenterOpacity (Utilities|Struct|BreakStruct_FlareItem _array_element)) (.LocOpacityEdgeOpacity (Utilities|Struct|BreakStruct_FlareItem _array_element)) (.LocOpacityInfluence (Utilities|Struct|BreakStruct_FlareItem _array_element))))))
    (Variables|/Game/LensFlareEff/Blueprints/FlareWidget.FlareWidget_C|SetOcclusion%20Update%20Speed (.FlareWidget (Utilities|Struct|BreakStruct_FlareItem (Utilities|Struct|MakeStruct_FlareItem (.Color (Utilities|Struct|BreakStruct_FlareItem _array_element)) _returnvalue (.FlareLocation (Utilities|Struct|BreakStruct_FlareItem _array_element)) (.IsMaterialAdditive (Utilities|Struct|BreakStruct_FlareItem _array_element)) (.FadeoutEdgeDistance (Utilities|Struct|BreakStruct_FlareItem _array_element)) (.ElementMaximumDistance (Utilities|Struct|BreakStruct_FlareItem _array_element)) (.FadeOut_EnableShrinking (Utilities|Struct|BreakStruct_FlareItem _array_element)) true (.FadeOut_FlareLocation (Utilities|Struct|BreakStruct_FlareItem _array_element)) (.Material (Utilities|Struct|BreakStruct_FlareItem _array_element)) (.ScreenPositionOffset (Utilities|Struct|BreakStruct_FlareItem _array_element)) (.GlobalSizeMultiplier (Utilities|Struct|BreakStruct_FlareItem _array_element)) (.InitialSpriteAngle (Utilities|Struct|BreakStruct_FlareItem _array_element)) (.ActiveRotationAmount (Utilities|Struct|BreakStruct_FlareItem _array_element)) (.EnableOrbitRotation (Utilities|Struct|BreakStruct_FlareItem _array_element)) (.EnablesLocationScaling (Utilities|Struct|BreakStruct_FlareItem _array_element)) (.LocationScalingInfluence (Utilities|Struct|BreakStruct_FlareItem _array_element)) (.LocationScalingCenterSize (Utilities|Struct|BreakStruct_FlareItem _array_element)) (.LocationScalingEdgeSize (Utilities|Struct|BreakStruct_FlareItem _array_element)) (.EnableLocationBasedOpacity (Utilities|Struct|BreakStruct_FlareItem _array_element)) (.LocOpacityCenterOpacity (Utilities|Struct|BreakStruct_FlareItem _array_element)) (.LocOpacityEdgeOpacity (Utilities|Struct|BreakStruct_FlareItem _array_element)) (.LocOpacityInfluence (Utilities|Struct|BreakStruct_FlareItem _array_element))))) (Variables|Global|GetOcclusion%20Update%20Speed))
    (Variables|Default|SetlightColor (Math|Conversions|ToColor(LinearColor) (.SpecifiedColor (Utilities|Struct|BreakSlateColor (.Color (Utilities|Struct|BreakStruct_FlareItem (Utilities|Struct|MakeStruct_FlareItem (.Color (Utilities|Struct|BreakStruct_FlareItem (Utilities|Array|Get(acopy) _flare_elements))) 0 1.0 true "(X=300.000000,Y=50.000000)" 5e+03 false true false 0)))))))))

(fn GetLocalCharacterCameraLocation
  (params (WorldContextObject :type Object%20Object%20Reference))
  (return (CallFunction|GetLocalCharacterCameraLocation WorldContextObject)))