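; Paintable plane actor that draws a brush stroke into a render target whenever it receives point damage.
; The construction script creates dynamic instances of a display material for the plane and a separate paint material.
; On damage, it writes brush size, strength and the ShotFromDirection vector, used as brush position, to a material parameter collection, then draws the paint material to the canvas render target.
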(event Game|Damage|EventPointDamage
  (params (Damage :type Float%20%28single-precision%29) (DamageType :type Damage%20Type%20Object%20Reference) (HitLocation :type Vector :default "0, 0, 0") (HitNormal :type Vector :default "0, 0, 0") (HitComponent :type Primitive%20Component%20Object%20Reference) (BoneName :type Name :default "None") (ShotFromDirection :type Vector :default "0, 0, 0") (InstigatedBy :type Controller%20Object%20Reference) (DamageCauser :type Actor%20Object%20Reference) (HitInfo :type Hit%20Result%20Structure%20%28by%20ref%29))
  (Rendering|Material|SetScalarParameterValue "/Game/Sector_Fusing/PaintMat_Col.PaintMat_Col" "ForceSize" (Variables|Default|GetBrushSize) :!class /Script/Engine.KismetMaterialLibrary)
  (Rendering|Material|SetScalarParameterValue "/Game/Sector_Fusing/PaintMat_Col.PaintMat_Col" "ForceStrength" (Variables|Default|GetBrushStrength) :!class /Script/Engine.KismetMaterialLibrary)
  (Rendering|Material|SetVectorParameterValue "/Game/Sector_Fusing/PaintMat_Col.PaintMat_Col" "ForcePos" (Math|Conversions|ToLinearColor(Vector) ShotFromDirection) :!class /Script/Engine.KismetMaterialLibrary)
  (Rendering|DrawMaterialtoRenderTarget "/Game/Sector_Fusing/NewCanvasRenderTarget2D.NewCanvasRenderTarget2D" (Variables|Default|GetPaintMat)))

(fn ConstructionScript
  (bind _returnvalue (Rendering|Material|CreateDynamicMaterialInstance "/Game/Sector_Fusing/Standard_M_Inst.Standard_M_Inst" "None" :!class /Script/Engine.KismetMaterialLibrary))
  (Variables|Default|SetPlaneMat _returnvalue)
  (Rendering|Material|SetMaterial (Variables|Actor|GetPlane) 0 _returnvalue)
  (bind _returnvalue_2 (Rendering|Material|CreateDynamicMaterialInstance "/Game/Sector_Fusing/Paint_M.Paint_M" "None" :!class /Script/Engine.KismetMaterialLibrary))
  (Variables|Default|SetPaintMat _returnvalue_2))